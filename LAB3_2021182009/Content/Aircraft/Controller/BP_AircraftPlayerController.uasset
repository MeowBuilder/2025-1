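; Player controller for an aircraft pawn that handles flight input and spawns high-speed effects.
; It adds the aircraft mapping context on BeginPlay, with Enhanced Input actions driving yaw, pitch and forward/right movement.
; Translation input scales with capped hold time, which is also stored as Speed.
; Each Tick, Speedy spawns two small explosion emitters at world-X offsets around the pawn while Speed exceeds a threshold.
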(event Input|EnhancedActionEvents|EnhancedInputActionIA_RotateAitcraft
  (params (ActionValue :type Vector%202D%20Structure) (ElapsedSeconds :type Float%20%28double-precision%29) (TriggeredSeconds :type Float%20%28double-precision%29) (InputAction :type Input%20Action%20Object%20Reference :default "/Game/Aircraft/Controller/IA_RotateAitcraft.IA_RotateAitcraft"))
  (Class|PlayerController|AddYawInput (.x ActionValue))
  (Class|PlayerController|AddPitchInput (.y ActionValue)))

(event Input|EnhancedActionEvents|EnhancedInputActionIA_TranslateAircraft
  (params (ActionValue :type Vector%202D%20Structure) (ElapsedSeconds :type Float%20%28double-precision%29) (TriggeredSeconds :type Float%20%28double-precision%29) (InputAction :type Input%20Action%20Object%20Reference :default "/Game/Aircraft/Controller/IA_TranslateAircraft.IA_TranslateAircraft"))
  (bind _returnvalue (Pawn|GetControlledPawn))
  (bind _returnvalue_2 (Math|Float|Min(Float) TriggeredSeconds 1e+01))
  (Variables|Default|Setspeed _returnvalue_2)
  (Pawn|Input|AddMovementInput _returnvalue (Transformation|GetActorForwardVector _returnvalue) (* (.x ActionValue) _returnvalue_2) false)
  (Pawn|Input|AddMovementInput _returnvalue (Transformation|GetActorRightVector _returnvalue) (* _returnvalue_2 (.y ActionValue)) false))

(event EventBeginPlay
  (Input|AddMappingContext (PlayerController|LocalPlayerSubsystems|GetEnhancedInputLocalPlayerSubsystem) "/Game/Aircraft/Controller/IMC_AircraftControl.IMC_AircraftControl" 0 "(bIgnoreAllPressedKeysUntilRelease=True,bForceImmediately=False,bNotifyUserSettings=False)"))

(event EventTick
  (params (DeltaSeconds :type Float%20%28single-precision%29))
  (CallFunction|Speedy (Pawn|GetControlledPawn)))

(fn ConstructionScript)

(fn Speedy
  (params (self2 :type Actor%20Object%20Reference))
  (bind _returnvalue (Transformation|GetActorLocation self2))
  (if (> (Variables|Default|Getspeed) 8.5)
    (Effects|SpawnEmitteratLocation "/Game/StarterContent/Particles/P_Explosion.P_Explosion" (+ _returnvalue "50.000000,0.000000,0.000000") "0.000000,0.000000,0.000000" "0.100000,0.100000,0.100000")
    (Effects|SpawnEmitteratLocation "/Game/StarterContent/Particles/P_Explosion.P_Explosion" (+ _returnvalue "-50.000000,0.000000,0.000000") "0, 0, 0" "0.100000,0.100000,0.100000")))